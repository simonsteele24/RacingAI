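; BP_Follow is the track-following state for hatchback AI controllers, with its own update and transition check.
; Update copies steering and throttle from the Path, capped by the car's AI speed, into the controller.
; CheckForTransition switches state when the current checkpoint is no longer ahead, a nearby car is behind (blocking), or a forward trace finds a car to pass.
; Dot products decide ahead or behind; debug trace drawing and a "Hello" print remain.
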(fn `CheckForTransition`
  (params (Controller :type "/Game/VehicleVarietyPack/Blueprints/Hatchback/BP_Hatchback_AIController Object Reference"))
  (returns (ReturnedState :type "/Game/VehicleVarietyPack/Blueprints/Hatchback/ENUM_State Enum"))
  (bind _returnvalue (`Controller.K2_GetPawn` Controller))
  (bind _car (`/Game/VehicleVarietyPack/Blueprints/Hatchback/BP_Hatchback_AIController.Car` Controller))
  (bind _car_2 (`/Game/VehicleVarietyPack/Blueprints/Hatchback/BP_Hatchback_AIController.Car` Controller))
  (bind _returnvalue_2 (`self.K2_GetActorLocation` _car_2))
  (bind _returnvalue_3 (+ (* (`self.GetActorUpVector` _car) 100.0) (`self.K2_GetActorLocation` _car)))
  (if (<= (`KismetMathLibrary.Dot_VectorVector` (- (`self.K2_GetActorLocation` (`BlueprintMapLibrary.Map_Find` (`/Game/VehicleVarietyPack/Blueprints/Hatchback/BP_Hatchback_AIController.Checkpoints` Controller) (`/Game/VehicleVarietyPack/Blueprints/Hatchback/BP_Hatchback_AIController.CurrentCheckPointNum` Controller))) (`self.K2_GetActorLocation` _returnvalue)) (`self.GetActorForwardVector` _returnvalue)) 0.0)
    (return "NewEnumerator4")
    (else
      (bind _outactors (`GameplayStatics.GetAllActorsOfClass` "/Game/VehicleVarietyPack/Blueprints/Hatchback/BP_Hatchback.BP_Hatchback_C"))
      (for _array_element _outactors
        (if (!= _array_element _car_2)
          (bind _returnvalue_4 (`self.K2_GetActorLocation` _array_element))
          (if (and (<= (`KismetMathLibrary.Vector_Distance` _returnvalue_4 _returnvalue_2) (`self.DistanceUntilBlock`)) (> 0.0 (`KismetMathLibrary.Dot_VectorVector` (- _returnvalue_4 _returnvalue_2) (`self.GetActorForwardVector` _car_2))))
            (set `/Game/VehicleVarietyPack/Blueprints/Hatchback/BP_Hatchback_AIController.CarToPass` _array_element Controller)
            (return "NewEnumerator2"))))
      (bind (_outhit _returnvalue_5) (`KismetSystemLibrary.LineTraceSingle` _returnvalue_3 (+ _returnvalue_3 (* (`self.GetActorForwardVector` _car) (`self.DistanceToCheckForPass`))) "TraceTypeQuery1" false (`|MakeArray` _car_2 :!type "Actor Object Reference") "ForOneFrame"))
      (if _returnvalue_5
        (bind _asbp_hatchback (cast `/Game/VehicleVarietyPack/Blueprints/Hatchback/BP_Hatchback` (`.HitActor` (`GameplayStatics.BreakHitResult` _outhit)))
          (:`then`
            (bind _asbp_hatchback_aicontroller (cast `/Game/VehicleVarietyPack/Blueprints/Hatchback/BP_Hatchback_AIController` (`Pawn.GetController` _asbp_hatchback))
              (:`then`
                (if (`|EnumInequality` (`/Game/VehicleVarietyPack/Blueprints/Hatchback/BP_Hatchback_AIController.CurrentState` _asbp_hatchback_aicontroller) "NewEnumerator1")
                  (`KismetSystemLibrary.PrintString` "Hello" :!label _label)
                  (set `/Game/VehicleVarietyPack/Blueprints/Hatchback/BP_Hatchback_AIController.CarToPass` _asbp_hatchback Controller)
                  (return "NewEnumerator1")
                  (else
                    _)))
              (:`CastFailed`
                (goto _label))))
          (:`CastFailed`
            _)))
      (return "NewEnumerator0"))))

(fn `Update`
  (params (OwnedPawn :type "/Game/VehicleVarietyPack/Blueprints/Hatchback/BP_Hatchback Object Reference") (Controller :type "/Game/VehicleVarietyPack/Blueprints/Hatchback/BP_Hatchback_AIController Object Reference") (Path :type "/Game/VehicleVarietyPack/Blueprints/Hatchback/SplineRFollow_Hatchback Object Reference"))
  (bind (_steering _throttle) (`/Game/VehicleVarietyPack/Blueprints/Hatchback/SplineRFollow_Hatchback.GetSteeringAndThrottleFromTrack` Path OwnedPawn (`/Game/VehicleVarietyPack/Blueprints/Hatchback/BP_Hatchback.AISpeed` OwnedPawn)))
  (set `/Game/VehicleVarietyPack/Blueprints/Hatchback/BP_Hatchback_AIController.Steering` _steering Controller)
  (set `/Game/VehicleVarietyPack/Blueprints/Hatchback/BP_Hatchback_AIController.AutoThrottle` _throttle Controller))

(fn `UserConstructionScript`
  (`parent.UserConstructionScript`))