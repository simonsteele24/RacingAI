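; Player controller for the hatchback vehicle that forwards driving and camera input to the car.
; On BeginPlay it casts player pawn 0 to BP_Hatchback and stores it as Car.
; Forward and right axes feed the car's acceleration and steering.
; The LookUp axis event drives camera control, reading the LookRight axis value alongside its own.
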(event `self.ReceiveBeginPlay`
  (bind _asbp_new_hatchback (cast `/Game/VehicleVarietyPack/Blueprints/Hatchback/BP_Hatchback` (`GameplayStatics.GetPlayerPawn` 0)))
  (set `self.Car` _asbp_new_hatchback))

(event `InputAxis|MoveForward`
  (params (AxisValue :type "Float (single-precision)"))
  (`MyHatchback.AddToAcceleration` (`self.Car`) AxisValue))

(event `InputAxis|MoveRight`
  (params (AxisValue :type "Float (single-precision)"))
  (`MyHatchback.AddToSteering` (`self.Car`) AxisValue))

(event `InputAxis|LookUp`
  (params (AxisValue :type "Float (single-precision)"))
  (`MyHatchback.ControlCamera` (`self.Car`) AxisValue (`self.GetInputAxisValue`)))

(fn `UserConstructionScript`)