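; BP_Pass is an AI driving state that steers a car around another car and back onto its path.
; Update first targets a side offset from CarToPass, then the path point closest to a spot along that car's forward axis, with throttle from AISpeed.
; CheckForTransition uses planar distance to the target to flip HasMadePass and return the next state.
; Its line trace only draws persistent debug lines; the result is unused.
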(fn `CheckForTransition`
  (params (Controller :type "/Game/VehicleVarietyPack/Blueprints/Hatchback/BP_Hatchback_AIController Object Reference"))
  (returns (ReturnedState :type "/Game/VehicleVarietyPack/Blueprints/Hatchback/ENUM_State Enum"))
  (bind (_steering_x _steering_y) (`KismetMathLibrary.BreakVector` (`/Game/VehicleVarietyPack/Blueprints/Hatchback/BP_Hatchback_AIController.Steering` Controller)))
  (bind (_steering_x_2 _steering_y_2) (`KismetMathLibrary.BreakVector` (`/Game/VehicleVarietyPack/Blueprints/Hatchback/BP_Hatchback_AIController.Steering` Controller)))
  (bind (_returnvalue_x _returnvalue_y) (`KismetMathLibrary.BreakVector` (`self.K2_GetActorLocation` (`/Game/VehicleVarietyPack/Blueprints/Hatchback/BP_Hatchback_AIController.Car` Controller))))
  (bind (_returnvalue_x_2 _returnvalue_y_2) (`KismetMathLibrary.BreakVector` (`self.K2_GetActorLocation` (`/Game/VehicleVarietyPack/Blueprints/Hatchback/BP_Hatchback_AIController.Car` Controller))))
  (`KismetSystemLibrary.LineTraceSingle` :`Start` (`self.K2_GetActorLocation` (`/Game/VehicleVarietyPack/Blueprints/Hatchback/BP_Hatchback_AIController.Car` Controller)) :`End` (`/Game/VehicleVarietyPack/Blueprints/Hatchback/BP_Hatchback_AIController.Steering` Controller) :`TraceChannel` "TraceTypeQuery1" :`DrawDebugType` "Persistent")
  (if (`self.HasMadePass`)
    (if (<= (`KismetMathLibrary.Vector_Distance` (`KismetMathLibrary.MakeVector` _steering_x _steering_y) (`KismetMathLibrary.MakeVector` _returnvalue_x _returnvalue_y)) (`self.DistanceToStopPass`))
      (set `self.HasMadePass` false)
      (return "NewEnumerator0")
      (else
        _))
    (elif (<= (`KismetMathLibrary.Vector_Distance` (`KismetMathLibrary.MakeVector` _steering_x_2 _steering_y_2) (`KismetMathLibrary.MakeVector` _returnvalue_x_2 _returnvalue_y_2)) (`self.DistanceToTurnBackOntoLine`))
      (set `self.HasMadePass` true)))
  (return "NewEnumerator1"))

(fn `Update`
  (params (OwnedPawn :type "/Game/VehicleVarietyPack/Blueprints/Hatchback/BP_Hatchback Object Reference") (Controller :type "/Game/VehicleVarietyPack/Blueprints/Hatchback/BP_Hatchback_AIController Object Reference") (Path :type "/Game/VehicleVarietyPack/Blueprints/Hatchback/SplineRFollow_Hatchback Object Reference"))
  (bind _cartopass (`/Game/VehicleVarietyPack/Blueprints/Hatchback/BP_Hatchback_AIController.CarToPass` Controller))
  (bind (_returnvalue_x _returnvalue_y) (`KismetMathLibrary.BreakVector` (`self.K2_GetActorLocation` _cartopass)))
  (if (`self.HasMadePass`)
    (set `/Game/VehicleVarietyPack/Blueprints/Hatchback/BP_Hatchback_AIController.Steering` (`SplineComponent.FindLocationClosestToWorldLocation` (`/Game/VehicleVarietyPack/Blueprints/Hatchback/SplineRFollow_Hatchback.Path` Path) (+ (`KismetMathLibrary.MakeVector` _returnvalue_x _returnvalue_y -140.0) (* (`self.GetActorForwardVector` _cartopass) (`self.ReturnToLine`))) "World") Controller)
    (else
      (set `/Game/VehicleVarietyPack/Blueprints/Hatchback/BP_Hatchback_AIController.Steering` (+ (`self.K2_GetActorLocation` _cartopass) (* (`self.GetActorRightVector` _cartopass) (`self.WidthOfPass`))) Controller)))
  (set `/Game/VehicleVarietyPack/Blueprints/Hatchback/BP_Hatchback_AIController.AutoThrottle` (`/Game/VehicleVarietyPack/Blueprints/Hatchback/BP_Hatchback.AISpeed` OwnedPawn) Controller))

(fn `UserConstructionScript`
  (`parent.UserConstructionScript`))