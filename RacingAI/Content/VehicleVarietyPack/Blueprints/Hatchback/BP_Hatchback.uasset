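; BP_Hatchback is a drivable hatchback vehicle pawn that exposes functions for driving and camera control.
; Throttle, steering and handbrake functions pass their values straight to the VehicleMovement component.
; The camera function feeds look axes into controller pitch and yaw, inverting pitch.
; Every tick it applies a world-vertical force scaled by GravityStrength to the mesh, acting as a gravity adjustment.
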(event `self.ReceiveTick`
  (params (DeltaSeconds :type "Float (single-precision)"))
  (`PrimitiveComponent.AddForce` (`self.Mesh`) (* (`KismetMathLibrary.GetUpVector` (struct)) (`self.GravityStrength`)) "None" false))

(fn `AddToAcceleration`
  (params (NewAxisVal :type "Float (double-precision)"))
  (`WheeledVehicleMovementComponent.SetThrottleInput` (`self.VehicleMovement`) NewAxisVal))

(fn `AddToSteering`
  (params (SteeringInput :type "Float (double-precision)"))
  (`WheeledVehicleMovementComponent.SetSteeringInput` (`self.VehicleMovement`) SteeringInput))

(fn `Brake`
  (params (`IsBraking?` :type Boolean))
  (`WheeledVehicleMovementComponent.SetHandbrakeInput` (`self.VehicleMovement`) `IsBraking?`))

(fn `ControlCamera`
  (params (LookUpAxis :type "Float (double-precision)") (LookRightAxis :type "Float (double-precision)"))
  (`self.AddControllerPitchInput` (* LookUpAxis -1.0))
  (`self.AddControllerYawInput` LookRightAxis))

(fn `UserConstructionScript`)